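; BP_Axe is a VR throwable axe that hits and destroys BP_Target_Base actors its box overlaps, destroying itself too if already thrown.
; BP_GrabComponent events toggle input and the holding hand's visibility message, sent to the motion controller's owner to avoid a hard VR pawn reference.
; On release it adds a fixed-strength impulse along its velocity, asks AxeSpawner for a replacement and destroys itself after a delay.
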(event OnComponentBeginOverlap(Box)
  (params (OverlappedComponent :type Primitive%20Component%20Object%20Reference) (OtherActor :type Actor%20Object%20Reference) (OtherComp :type Primitive%20Component%20Object%20Reference) (OtherBodyIndex :type Integer) (bFromSweep :type Boolean) (SweepResult :type Hit%20Result%20Structure%20%28by%20ref%29))
  (bind _asbp_target_base (Utilities|Casting|CastToBP_Target_Base OtherActor))
  (if (Variables|Default|GetHasBeenThrown)
    (Actor|DestroyActor))
  (Default|GetHit _asbp_target_base)
  (Actor|DestroyActor _asbp_target_base))

(event OnDropped(BP_GrabComponent)
  (bind _bp_grabcomponent (Variables|Default|GetBP_GrabComponent))
  (Input|DisableInput (Game|GetPlayerController 0))
  (Class|BPIPawnAnim|HideUnhideHand(Message) (Components|GetOwner (Variables|/Game/XRFramework/Blueprints/BP_GrabComponent.BP_GrabComponent_C|GetMotionControllerRef _bp_grabcomponent)) false (Utilities|Enum|Equal(Enum) (Default|GetHeldbyHand _bp_grabcomponent) "Right"))
  (Variables|Default|SetHasBeenThrown true)
  (bind _returnvalue (Physics|GetPhysicsLinearVelocity (Variables|Default|GetAxeMesh) "None"))
  (Physics|AddImpulse (Variables|Default|GetAxeMesh) (* (Math|Vector|Normalize _returnvalue) "2000.000000,2000.000000,2000.000000") "None" false)
  (Default|SpawnAxe (Variables|Default|GetAxeSpawner))
  (Utilities|FlowControl|Delay 5.0)
  (Actor|DestroyActor))

(event OnGrabbed(BP_GrabComponent)
  (bind _bp_grabcomponent (Variables|Default|GetBP_GrabComponent))
  (Input|EnableInput (Game|GetPlayerController 0))
  (Class|BPIPawnAnim|HideUnhideHand(Message) (Components|GetOwner (Variables|/Game/XRFramework/Blueprints/BP_GrabComponent.BP_GrabComponent_C|GetMotionControllerRef _bp_grabcomponent)) true (Utilities|Enum|Equal(Enum) (Default|GetHeldbyHand _bp_grabcomponent) "Right")))

(event EventBeginPlay)

(event EventTick
  (params (DeltaSeconds :type Float%20%28single-precision%29)))

(fn ConstructionScript)