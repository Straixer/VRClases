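; BP_Pistol is a grabbable VR pistol with separate shoot and reload inputs for each hand, calling shared left and right weapon functions.
; Each trigger press fires once, with the firing flag raised only around the shoot call.
; Grabbing enables input, adds the holding hand's weapon mapping context and hides that hand via the motion controller's owner, avoiding a hard VR Pawn reference.
; Dropping reverses all three.
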(event OnGrabbed(GrabComponentSnap)
  (bind _grabcomponentsnap (Variables|Default|GetGrabComponentSnap))
  (bind _returnvalue (Default|GetHeldbyHand _grabcomponentsnap))
  (bind _returnvalue_2 (Utilities|Enum|Equal(Enum) _returnvalue "Right"))
  (Input|EnableInput (Game|GetPlayerController 0))
  (Class|BPIPawnAnim|HideUnhideHand(Message) (Components|GetOwner (Variables|/Game/XRFramework/Blueprints/BP_GrabComponent.BP_GrabComponent_C|GetMotionControllerRef _grabcomponentsnap)) true _returnvalue_2)
  (Input|AddMappingContext (PlayerController|LocalPlayerSubsystems|GetEnhancedInputLocalPlayerSubsystem (Game|GetPlayerController 0)) (select _returnvalue_2 "/Game/XRFramework/Input/IMC_Weapon_Right.IMC_Weapon_Right" "/Game/XRFramework/Input/IMC_Weapon_Left.IMC_Weapon_Left") 1 "(bIgnoreAllPressedKeysUntilRelease=True,bForceImmediately=False,bNotifyUserSettings=False)"))

(event OnDropped(GrabComponentSnap)
  (bind _grabcomponentsnap (Variables|Default|GetGrabComponentSnap))
  (bind _returnvalue (Default|GetHeldbyHand _grabcomponentsnap))
  (bind _returnvalue_2 (Utilities|Enum|Equal(Enum) _returnvalue "Right"))
  (Input|DisableInput (Game|GetPlayerController 0))
  (Class|BPIPawnAnim|HideUnhideHand(Message) (Components|GetOwner (Variables|/Game/XRFramework/Blueprints/BP_GrabComponent.BP_GrabComponent_C|GetMotionControllerRef _grabcomponentsnap)) false _returnvalue_2)
  (Input|RemoveMappingContext (PlayerController|LocalPlayerSubsystems|GetEnhancedInputLocalPlayerSubsystem (Game|GetPlayerController 0)) (select _returnvalue_2 "/Game/XRFramework/Input/IMC_Weapon_Right.IMC_Weapon_Right" "/Game/XRFramework/Input/IMC_Weapon_Left.IMC_Weapon_Left") "(bIgnoreAllPressedKeysUntilRelease=True,bForceImmediately=False,bNotifyUserSettings=False)"))

(event Input|EnhancedActionEvents|EnhancedInputActionIA_Shoot_Left
  (params (ActionValue :type Boolean) (ElapsedSeconds :type Float%20%28double-precision%29) (TriggeredSeconds :type Float%20%28double-precision%29) (InputAction :type Input%20Action%20Object%20Reference :default "/Game/XRFramework/Input/Actions/IA_Shoot_Left.IA_Shoot_Left"))
  (:Started
    (Variables|Default|SetIsFiringLeft true)
    (CallFunction|ShootLeft)
    (Variables|Default|SetIsFiringLeft false)))

(event Input|EnhancedActionEvents|EnhancedInputActionIA_Shoot_Right
  (params (ActionValue :type Boolean) (ElapsedSeconds :type Float%20%28double-precision%29) (TriggeredSeconds :type Float%20%28double-precision%29) (InputAction :type Input%20Action%20Object%20Reference :default "/Game/XRFramework/Input/Actions/IA_Shoot_Right.IA_Shoot_Right"))
  (:Started
    (Variables|Default|SetIsFiringRight true)
    (CallFunction|ShootRight)
    (Variables|Default|SetIsFiringRight false)))

(event Input|EnhancedActionEvents|EnhancedInputActionIA_Reload_Left
  (params (ActionValue :type Boolean) (ElapsedSeconds :type Float%20%28double-precision%29) (TriggeredSeconds :type Float%20%28double-precision%29) (InputAction :type Input%20Action%20Object%20Reference :default "/Game/XRFramework/Input/Actions/IA_Reload_Left.IA_Reload_Left"))
  (:Started
    (CallFunction|ReloadLeft)))

(event Input|EnhancedActionEvents|EnhancedInputActionIA_Reload_Right
  (params (ActionValue :type Boolean) (ElapsedSeconds :type Float%20%28double-precision%29) (TriggeredSeconds :type Float%20%28double-precision%29) (InputAction :type Input%20Action%20Object%20Reference :default "/Game/XRFramework/Input/Actions/IA_Reload_Right.IA_Reload_Right"))
  (:Started
    (CallFunction|ReloadRight)))

(fn ConstructionScript
  (|CallParentFunction))