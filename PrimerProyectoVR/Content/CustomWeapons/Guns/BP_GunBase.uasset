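; BP_GunBase is a VR gun base that fires projectiles from its muzzle and supports timed reloading.
; Separate left and right shoot and reload events act only when GrabComponentSnap reports that hand is holding it.
; Each shot spawns ProjectileClass, plays haptics, decrements ammo and updates the ammo display.
; Automatic fire comes from each shoot event re-calling itself after FireRate while its firing flag, ammo and reload state allow.
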(event Custom|ReloadLeft
  (if (Utilities|Enum|Equal(Enum) (Default|GetHeldbyHand (Variables|Default|GetGrabComponentSnap)) "Left")
    (Variables|Default|SetReloading true)
    (Utilities|FlowControl|Delay (Variables|Default|GetReloadTime))
    (bind _output_get (Variables|Default|SetCurrentAmmo (Variables|Default|GetMaxAmmo)))
    (Rendering|Components|TextRender|SetText (Variables|Default|GetAmmoDisplay) (Utilities|Text|ToText(Integer) _output_get))
    (Variables|Default|SetReloading false)))

(event Custom|ReloadRight
  (if (Utilities|Enum|Equal(Enum) (Default|GetHeldbyHand (Variables|Default|GetGrabComponentSnap)) "Right")
    (Variables|Default|SetReloading true)
    (Utilities|FlowControl|Delay (Variables|Default|GetReloadTime))
    (bind _output_get (Variables|Default|SetCurrentAmmo (Variables|Default|GetMaxAmmo)))
    (Rendering|Components|TextRender|SetText (Variables|Default|GetAmmoDisplay) (Utilities|Text|ToText(Integer) _output_get))
    (Variables|Default|SetReloading false)))

(event Custom|ShootLeft
  (bind _muzzlelocation (Variables|Default|GetMuzzleLocation))
  (if (Utilities|Enum|Equal(Enum) (Default|GetHeldbyHand (Variables|Default|GetGrabComponentSnap)) "Left")
    (if (Variables|Default|GetIsFiringLeft)
      (if (not (Variables|Default|GetReloading))
        (if (> (Variables|Default|GetCurrentAmmo) 0)
          (Game|SpawnActorfromClass (Variables|Default|GetProjectileClass) (Math|Transform|MakeTransform (Transformation|GetWorldLocation _muzzlelocation) (Transformation|GetWorldRotation _muzzlelocation)) "Undefined" "OverrideRootScale" self (Game|Player|GetPlayerPawn 0))
          (Class|PlayerController|PlayHapticEffect (Game|GetPlayerController 0) (Variables|Default|GetPistolFireHapticEffect) (Default|GetHeldbyHand (Variables|Default|GetGrabComponentSnap)) 1.0 false)
          (if (> (Variables|Default|GetCurrentAmmo) 0)
            (bind _output_get (Variables|Default|SetCurrentAmmo (- (Variables|Default|GetCurrentAmmo) 1)))
            (Rendering|Components|TextRender|SetText (Variables|Default|GetAmmoDisplay) (Utilities|Text|ToText(Integer) _output_get))
            (Utilities|FlowControl|Delay (Variables|Default|GetFireRate))
            (CallFunction|ShootLeft)))))))

(event Custom|ShootRight
  (bind _muzzlelocation (Variables|Default|GetMuzzleLocation))
  (if (Utilities|Enum|Equal(Enum) (Default|GetHeldbyHand (Variables|Default|GetGrabComponentSnap)) "Right")
    (if (Variables|Default|GetIsFiringRight)
      (if (not (Variables|Default|GetReloading))
        (if (> (Variables|Default|GetCurrentAmmo) 0)
          (Game|SpawnActorfromClass (Variables|Default|GetProjectileClass) (Math|Transform|MakeTransform (Transformation|GetWorldLocation _muzzlelocation) (Transformation|GetWorldRotation _muzzlelocation)) "Undefined" "OverrideRootScale" self (Game|Player|GetPlayerPawn 0))
          (Class|PlayerController|PlayHapticEffect (Game|GetPlayerController 0) (Variables|Default|GetPistolFireHapticEffect) (Default|GetHeldbyHand (Variables|Default|GetGrabComponentSnap)) 1.0 false)
          (if (> (Variables|Default|GetCurrentAmmo) 0)
            (bind _output_get (Variables|Default|SetCurrentAmmo (- (Variables|Default|GetCurrentAmmo) 1)))
            (Rendering|Components|TextRender|SetText (Variables|Default|GetAmmoDisplay) (Utilities|Text|ToText(Integer) _output_get))
            (Utilities|FlowControl|Delay (Variables|Default|GetFireRate))
            (CallFunction|ShootRight)))))))

(fn ConstructionScript)