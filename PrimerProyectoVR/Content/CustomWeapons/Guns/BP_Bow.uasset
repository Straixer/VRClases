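; VR bow weapon that the player grabs in one hand and charges with the other hand's shoot input to fire arrows.
; Grabbing enables input, hides that hand's mesh message via HideUnhideHandMessage and adds the opposite hand's Enhanced Input mapping context; dropping reverses this.
; Pressing starts a looping timer that builds capped charge time.
; Releasing maps charge to speed and spawns BP_Arrow at the muzzle with that velocity.
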(event OnGrabbed(GrabComponentSnap)
  (bind _grabcomponentsnap (Variables|Default|GetGrabComponentSnap))
  (bind _returnvalue (Default|GetHeldbyHand _grabcomponentsnap))
  (bind _returnvalue_2 (Utilities|Enum|Equal(Enum) _returnvalue "Right"))
  (Input|EnableInput (Game|GetPlayerController 0))
  (Class|BPIPawnAnim|HideUnhideHand(Message) (Components|GetOwner (Variables|/Game/XRFramework/Blueprints/BP_GrabComponent.BP_GrabComponent_C|GetMotionControllerRef _grabcomponentsnap)) true _returnvalue_2)
  (Input|AddMappingContext (PlayerController|LocalPlayerSubsystems|GetEnhancedInputLocalPlayerSubsystem (Game|GetPlayerController 0)) (select _returnvalue_2 "/Game/XRFramework/Input/IMC_Weapon_Left.IMC_Weapon_Left" "/Game/XRFramework/Input/IMC_Weapon_Right.IMC_Weapon_Right") 1 "(bIgnoreAllPressedKeysUntilRelease=True,bForceImmediately=False,bNotifyUserSettings=False)"))

(event OnDropped(GrabComponentSnap)
  (bind _grabcomponentsnap (Variables|Default|GetGrabComponentSnap))
  (bind _returnvalue (Default|GetHeldbyHand _grabcomponentsnap))
  (bind _returnvalue_2 (Utilities|Enum|Equal(Enum) _returnvalue "Right"))
  (Input|DisableInput (Game|GetPlayerController 0))
  (Class|BPIPawnAnim|HideUnhideHand(Message) (Components|GetOwner (Variables|/Game/XRFramework/Blueprints/BP_GrabComponent.BP_GrabComponent_C|GetMotionControllerRef _grabcomponentsnap)) false _returnvalue_2)
  (Input|RemoveMappingContext (PlayerController|LocalPlayerSubsystems|GetEnhancedInputLocalPlayerSubsystem (Game|GetPlayerController 0)) (select _returnvalue_2 "/Game/XRFramework/Input/IMC_Weapon_Left.IMC_Weapon_Left" "/Game/XRFramework/Input/IMC_Weapon_Right.IMC_Weapon_Right") "(bIgnoreAllPressedKeysUntilRelease=True,bForceImmediately=False,bNotifyUserSettings=False)"))

(event Input|EnhancedActionEvents|EnhancedInputActionIA_Shoot_Left
  (params (ActionValue :type Boolean) (ElapsedSeconds :type Float%20%28double-precision%29) (TriggeredSeconds :type Float%20%28double-precision%29) (InputAction :type Input%20Action%20Object%20Reference :default "/Game/XRFramework/Input/Actions/IA_Shoot_Left.IA_Shoot_Left"))
  (:Started
    (Development|PrintString "Hello")
    (if (Utilities|Enum|Equal(Enum) (Default|GetHeldbyHand (Variables|Default|GetGrabComponentSnap)) "Right")
      (CallFunction|HandleShootPressed)))
  (:Completed
    (CallFunction|HandleShootReleased)))

(event Input|EnhancedActionEvents|EnhancedInputActionIA_Shoot_Right
  (params (ActionValue :type Boolean) (ElapsedSeconds :type Float%20%28double-precision%29) (TriggeredSeconds :type Float%20%28double-precision%29) (InputAction :type Input%20Action%20Object%20Reference :default "/Game/XRFramework/Input/Actions/IA_Shoot_Right.IA_Shoot_Right"))
  (:Started
    (if (Utilities|Enum|Equal(Enum) (Default|GetHeldbyHand (Variables|Default|GetGrabComponentSnap)) "Left")
      (CallFunction|HandleShootPressed)))
  (:Completed
    (CallFunction|HandleShootReleased)))

(fn ConstructionScript
  (|CallParentFunction))

(fn HandleShootPressed
  (Variables|Default|SetChargeTime 0.0)
  (Variables|Default|SetIsCharging true)
  (Utilities|Time|SetTimerbyFunctionName 0 "UpdateCharge" 0.1 true))

(fn HandleShootReleased
  (bind _muzzlelocation (Variables|Default|GetMuzzleLocation))
  (Variables|Default|SetIsCharging false)
  (Utilities|Time|ClearTimerbyFunctionName 0 "UpdateCharge")
  (Variables|Default|SetArrowSpeed (Math|Float|MapRangeClamped (Variables|Default|GetChargeTime) 0.0 (Variables|Default|GetMaxChargeTime) (Variables|Default|GetMinArrowSpeed) (Variables|Default|GetMaxArrowSpeed)))
  (bind _returnvalue (Game|SpawnActorfromClass "/Game/CustomWeapons/Projectiles/BP_Arrow.BP_Arrow_C" (Math|Transform|MakeTransform (Transformation|GetWorldLocation _muzzlelocation) (Transformation|GetWorldRotation _muzzlelocation)) "Undefined" "MultiplyWithRoot" self (Game|Player|GetPlayerPawn 0)))
  (Game|Components|ProjectileMovement|SetVelocityinLocalSpace (Variables|/Game/CustomWeapons/Projectiles/BP_Projectile.BP_Projectile_C|GetProjectileMovement _returnvalue) (Math|Conversions|ToVector(Float) (Variables|Default|GetArrowSpeed)))
  (Development|PrintString (Utilities|String|ToString(Float) (Variables|Default|GetArrowSpeed))))

(fn UpdateCharge
  (Variables|Default|SetChargeTime (Math|Float|Min(Float) (+ (Variables|Default|GetChargeTime) 0.1) (Variables|Default|GetMaxChargeTime))))