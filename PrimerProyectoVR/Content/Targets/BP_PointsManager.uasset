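; BP_PointsManager is an actor that tracks the player's score for kills of target enemies and allies.
; EnemyKilled adds points and AllyKilled subtracts a smaller penalty.
; Both functions then write the formatted total to the PointsRender text.
; The event graph and construction script are empty, so the score changes only through these two functions.
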(event EventBeginPlay)

(event Collision|EventActorBeginOverlap
  (params (OtherActor :type Actor%20Object%20Reference)))

(event EventTick
  (params (DeltaSeconds :type Float%20%28single-precision%29)))

(fn ConstructionScript)

(fn AllyKilled
  (bind _output_get (Variables|Default|SetPoints (- (Variables|Default|GetPoints) 2)))
  (Rendering|Components|TextRender|SetText (Variables|Default|GetPointsRender) (Utilities|Text|FormatText "Points: {Points}" _output_get)))

(fn EnemyKilled
  (bind _output_get (Variables|Default|SetPoints (+ (Variables|Default|GetPoints) 10)))
  (Rendering|Components|TextRender|SetText (Variables|Default|GetPointsRender) (Utilities|Text|FormatText "Points: {Points}" _output_get)))